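; Terminal interactable item with a trigger sphere, a widget component for a hint, and hacking state.
; Pressing F creates a WG_Terminal_Base widget without range checks or adding it to the screen.
; Sphere overlaps only cast to BP_PlayerCharacter; the hint show/hide logic is disconnected, so the widget stays hidden after BeginPlay.
; HACKEAR sets Hackeado when CanPressF is true, but nothing here calls it or sets that flag.
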(event `Key|F`
  (params (Key :type "Key Structure"))
  (:`Pressed`
    (`|CreateWidget` "/Game/FirstPerson/Blueprints/Widgets/WG_Terminal_Base.WG_Terminal_Base_C")))

(event `self.Sphere.OnComponentBeginOverlap`
  (params (OverlappedComponent :type "PrimitiveComponent Object Reference") (OtherActor :type "Actor Object Reference") (OtherComp :type "PrimitiveComponent Object Reference") (OtherBodyIndex :type Integer) (bFromSweep :type Boolean) (SweepResult :type "HitResult Structure (by ref)"))
  (cast `/Game/FirstPerson/Blueprints/BP_PlayerCharacter` OtherActor))

(event `self.ReceiveBeginPlay`
  (`SceneComponent.SetVisibility` (`self.Widget`) false false))

(event `self.Sphere.OnComponentEndOverlap`
  (params (OverlappedComponent :type "PrimitiveComponent Object Reference") (OtherActor :type "Actor Object Reference") (OtherComp :type "PrimitiveComponent Object Reference") (OtherBodyIndex :type Integer))
  (cast `/Game/FirstPerson/Blueprints/BP_PlayerCharacter` OtherActor))

(fn `HACKEAR`
  (if (`self.CanPressF`)
    (set `self.Hackeado` true)))

(fn `UserConstructionScript`)