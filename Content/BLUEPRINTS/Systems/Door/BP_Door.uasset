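; Door actor that swings open and closed when its Interact event is called.
; An IsOpen flag selects between playing and reversing the DoorRotation timeline, whose DoorTL track drives the door's relative yaw.
; Any actor overlap creates and shows a new WG_Interact widget, and end overlap hides it without removing it from the viewport.
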(event `/Game/BLUEPRINTS/Systems/Door/BPI_Interact.Interact`
  (if (`self.IsOpen`)
    (set `self.IsOpen` false)
    (bind (_direction _doortl) (`Timeline|DoorRotation` :!via `Reverse` :!label _label)
      (:`Update`
        (`SceneComponent.K2_SetRelativeRotation` (`self.Door`) (`KismetMathLibrary.MakeRotator` 0.0 0.0 _doortl) false false)))
    (else
      (set `self.IsOpen` true)
      (goto _label))))

(event `self.ReceiveActorBeginOverlap`
  (params (OtherActor :type "Actor Object Reference"))
  (bind _returnvalue (`|CreateWidget` "/Game/BLUEPRINTS/Widgets/WG_Interact.WG_Interact_C"))
  (`UserWidget.AddToViewport` _returnvalue 0)
  (set `Widget.Visibility` "Visible" _returnvalue))

(event `self.ReceiveActorEndOverlap`
  (params (OtherActor :type "Actor Object Reference"))
  (set `Widget.Visibility` "Hidden" (stale `self.ReceiveActorBeginOverlap` _returnvalue)))

(fn `UserConstructionScript`)