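; BP_Terminal is an interactable, one-time hackable terminal that opens a terminal UI.
; Interact acts only while Status is "No Hackeada": it marks the terminal hacked and swaps its mesh to the checkpoint-on material.
; It then shows WG_Terminal, pauses the game and shows the cursor while keeping game-only input mode.
; ShowInfo supplies the hack prompt to the interact widget until the terminal is hacked.
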(event `/Game/BLUEPRINTS/Systems/Additional_Logic/I_Interactable.Interact`
  (bind _returnvalue (`GameplayStatics.GetPlayerController` 0))
  (switch `/Game/BLUEPRINTS/Systems/Terminal/EN_Terminal_Hackeada` (`self.Status`)
    (:`NewEnumerator0`
      (set `self.Status` "NewEnumerator1")
      (`PrimitiveComponent.SetMaterial` (`self.StaticMesh`) 0 "/Game/BLUEPRINTS/Systems/Checkpoints/M_Checkpoint_On.M_Checkpoint_On")
      (bind _returnvalue_2 (`|CreateWidget` "/Game/BLUEPRINTS/Widgets/WG_Terminal.WG_Terminal_C"))
      (`UserWidget.AddToViewport` _returnvalue_2 0)
      (`WidgetBlueprintLibrary.SetInputMode_GameOnly` _returnvalue)
      (set `PlayerController.bShowMouseCursor` true _returnvalue)
      (`GameplayStatics.SetGamePaused` true))))

(event `/Game/BLUEPRINTS/Systems/Additional_Logic/I_Interactable.ShowInfo`
  (params (`WG Interact prompt` :type "/Game/BLUEPRINTS/Widgets/WG_Interact_Prompt Object Reference"))
  (switch `/Game/BLUEPRINTS/Systems/Terminal/EN_Terminal_Hackeada` (`self.Status`)
    (:`NewEnumerator0`
      (`/Game/BLUEPRINTS/Widgets/WG_Interact_Prompt.Set Info Text` `WG Interact prompt` "(F) Hack"))))

(fn `UserConstructionScript`)