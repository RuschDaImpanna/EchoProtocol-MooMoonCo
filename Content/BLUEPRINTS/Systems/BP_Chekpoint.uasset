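; BP_Chekpoint is a checkpoint actor that the player activates by walking into its trigger box.
; When the box overlaps player character 0, it swaps the static mesh material to the "on" checkpoint material.
; It then casts the game mode to BP_FirstPersonGameMode and stores itself as the current Checkpoint there.
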(event `Change to Green`
  (`PrimitiveComponent.SetMaterial` (`self.StaticMesh`) 0 "/Game/MAPS/MAP_1/MATERIALS/M_Chekpoint_On.M_Chekpoint_On"))

(event `self.Box.OnComponentBeginOverlap`
  (params (OverlappedComponent :type "PrimitiveComponent Object Reference") (OtherActor :type "Actor Object Reference") (OtherComp :type "PrimitiveComponent Object Reference") (OtherBodyIndex :type Integer) (bFromSweep :type Boolean) (SweepResult :type "HitResult Structure (by ref)"))
  (if (== OtherActor (`GameplayStatics.GetPlayerCharacter` 0))
    (`self.Change to Green`)
    (bind _asbp_first_person_game_mode (cast `/Game/FirstPerson/Blueprints/BP_FirstPersonGameMode` (`GameplayStatics.GetGameMode`)))
    (set `/Game/FirstPerson/Blueprints/BP_FirstPersonGameMode.Checkpoint` self _asbp_first_person_game_mode)))

(fn `UserConstructionScript`)