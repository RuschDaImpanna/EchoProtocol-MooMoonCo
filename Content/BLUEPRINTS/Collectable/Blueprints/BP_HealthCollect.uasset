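; BP_HealthCollect is a health pickup with a sci-fi med kit mesh that grants health to the player.
; Any box overlap calls HealthAssign on player character 0, without checking the overlapping actor.
; It then adds an audio component, sets the med kit visible and briefly raises the Niagara Flow parameter.
; After resetting the flow and waiting again, it calls KillMomentEvent, which is not defined in this graph.
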(event `self.Box.OnComponentBeginOverlap`
  (params (OverlappedComponent :type "PrimitiveComponent Object Reference") (OtherActor :type "Actor Object Reference") (OtherComp :type "PrimitiveComponent Object Reference") (OtherBodyIndex :type Integer) (bFromSweep :type Boolean) (SweepResult :type "HitResult Structure (by ref)"))
  (bind _niagara (`self.Niagara`))
  (bind _asbp_player_character (cast `/Game/FirstPerson/Blueprints/BP_PlayerCharacter` (`GameplayStatics.GetPlayerCharacter` 0)))
  (`/Game/FirstPerson/Blueprints/BP_PlayerCharacter.Health Assign` _asbp_player_character 10.0)
  (`AddComponent|NODE_AddAudioComponent-0`)
  (`SceneComponent.SetVisibility` (`self.Sci-fi_Med_kit`) true false)
  (`NiagaraComponent.SetVariableFloat` _niagara "Flow" 200.0)
  (`KismetSystemLibrary.Delay` 1.0)
  (`NiagaraComponent.SetVariableFloat` _niagara "Flow" 0.0)
  (`KismetSystemLibrary.Delay` 1.5)
  (`self.KillMoment_Event`))

(fn `UserConstructionScript`
  (`parent.UserConstructionScript`))